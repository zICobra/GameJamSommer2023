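; Game mode Blueprint that exposes menu-level events for audio settings, quitting and pause state.
; TriggerSettings creates a WBP_Audio widget, hides its background, adds it to the viewport and flags it as open.
; TriggerPause sets a state on PC_Firstperson and unpauses the game, despite its name, while ExitGame quits.
; GetIsUsingGamepad is hard-coded to return false.
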(event `/Game/UI/BPI_GameModeUI.TriggerSettings`
  ;[1 1 1] Comment
  (bind _returnvalue (`|CreateWidget` "/Game/UI/WBP_Audio.WBP_Audio_C"))
  (bind _output_get (set `self.AudioMenuRef` _returnvalue))
  (`Widget.SetVisibility` (`/Game/UI/WBP_Audio.BGAudio` _output_get) "Hidden")
  (`UserWidget.AddToViewport` _output_get 0)
  (set `self.IsAudioOn` true))

(event `/Game/UI/BPI_GameModeUI.ExitGame`
  ;[1 1 1] Comment
  (`KismetSystemLibrary.QuitGame` null "Quit"))

(event `/Game/UI/BPI_GameModeUI.TriggerPause`
  ;[1 1 1] Pause
  (bind _aspc_firstperson (cast `/Game/Blueprint/Character/PC_Firstperson` (`GameplayStatics.GetPlayerController` 0)))
  (`/Game/Blueprint/Character/PC_Firstperson.SetState` _aspc_firstperson "NewEnumerator0")
  (`GameplayStatics.SetGamePaused` false))

(fn `GetIsUsingGamepad`
  (returns (IsUsingGamepad :type Boolean))
  (return false))

(fn `UserConstructionScript`)